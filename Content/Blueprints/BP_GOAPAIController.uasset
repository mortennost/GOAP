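; BP_GOAPAIController is an AI controller that turns perception updates into GOAP world state.
; For each actor in an AI Perception update, it prints the actor's name and calls SetIsNearPlayer, which sets the IsNearPlayer atom to true if it is not already.
; The atom is never cleared here, and updated actors are not filtered for the player or for sensing success.
; A PawnSensing handler only prints debug text and is marked as not in use.
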(event `self.AIPerception.OnPerceptionUpdated`
  (params (UpdatedActors :type "Array of Actor Object Reference"))
  (for _array_element UpdatedActors
    (`KismetSystemLibrary.PrintString` (`KismetSystemLibrary.GetObjectName` _array_element) true true (struct :`R` 1.0 :`G` 0.775124 :`A` 1.0))
    (`self.SetIsNearPlayer`)))

(event `self.PawnSensing.OnSeePawn`
  (params (Pawn :type "Pawn Object Reference"))
  ;[1 1 1] PawnSensing debug (Not in use)
  (`KismetSystemLibrary.PrintString` (`KismetStringLibrary.Concat_StrStr` "PawnSensing: " (`KismetSystemLibrary.GetObjectName` Pawn)) true true (struct :`R` 0.296378 :`B` 0.405 :`A` 1.0)))

(fn `SetIsNearPlayer`
  (locals (IsNearPlayerAtom :type "GOAPAtom Structure" :default (struct :`Key` 1 :`Value` true)))
  (bind _goapatomkey (make `GOAPAtomKey` (`.Key` (break `GOAPAtom` (`local.IsNearPlayerAtom`)))))
  (bind _returnvalue (`self.GetWorldState` _goapatomkey))
  (if (not _returnvalue)
    (`self.SetWorldState` _goapatomkey true)))

(fn `UserConstructionScript`)