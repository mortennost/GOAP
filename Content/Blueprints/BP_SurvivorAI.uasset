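; BP_SurvivorAI is a GOAP-driven survivor AI that tracks hunger as planner world state.
; A looping timer lowers hunger through UpdateHunger, which clamps the value and flags IsHungry whenever it is below full.
; SetIsNearPlayer can cancel the current plan, stop movement and flag player proximity, but only disconnected nodes call it.
; AI Perception's update event is empty, and PawnSensing only prints debug text.
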(event `self.ReceiveBeginPlay`
  (`KismetSystemLibrary.K2_SetTimer` null "DecreaseHunger" 5.0 true))

(event `self.AIPerception.OnPerceptionUpdated`
  (params (UpdatedActors :type "Array of Actor Object Reference")))

(event `self.PawnSensing.OnSeePawn`
  (params (Pawn :type "Pawn Object Reference"))
  ;[1 1 1] PawnSensing debug (Not in use)
  (`KismetSystemLibrary.PrintString` (`KismetStringLibrary.Concat_StrStr` "PawnSensing: " (`KismetSystemLibrary.GetObjectName` Pawn)) true true (struct :`R` 0.296378 :`B` 0.405 :`A` 1.0)))

(fn `DecreaseHunger`
  (`self.UpdateHunger` -25))

(fn `SetIsNearPlayer`
  (locals (IsNearPlayerAtom :type "GOAPAtom Structure" :default (struct :`Key` 1 :`Value` true)))
  (bind _goapatomkey (make `GOAPAtomKey` (`.Key` (break `GOAPAtom` (`local.IsNearPlayerAtom`)))))
  (bind _returnvalue (`self.GetWorldState` _goapatomkey))
  (if (not _returnvalue)
    (`self.ClearCurrentActionAndPlan`)
    (`self.StopMovement`)
    (`self.SetWorldState` _goapatomkey true)))

(fn `UpdateHunger`
  (params (AddHunger :type Integer))
  (bind _output_get (set `self.HungerValue` (`KismetMathLibrary.Clamp` (+ (`self.HungerValue`) AddHunger) 0 100)))
  (`self.SetWorldState` (make `GOAPAtomKey` (`.Key` (break `GOAPAtom` (`self.IsHungryAtom`)))) (< _output_get 100)))

(fn `UserConstructionScript`)